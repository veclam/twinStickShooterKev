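; ReduceSpeed is a component that slows its owning projectile to a stop after a delay, part of the Stylized Slashes pack.
; On BeginPlay it caches the owner's ProjectileMovementComponent, if one exists, waits for the configured delay, then enables slowing.
; Tick then uses VInterpTo to ease the projectile's velocity toward zero at the configured rate.
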(event `self.ReceiveBeginPlay`
  (bind _returnvalue (`Actor.GetComponentByClass` (`self.GetOwner`) "/Script/Engine.ProjectileMovementComponent"))
  (`/Engine/EditorBlueprintResources/StandardMacros.IsValid` _returnvalue
    (:`Is Valid`
      (set `self.ProjectileMovement` _returnvalue)
      (`KismetSystemLibrary.Delay` (`self.Delay`))
      (set `self.ReduceSpeed` true))))

(event `self.ReceiveTick`
  (params (DeltaSeconds :type "Float (single-precision)"))
  (bind _projectilemovement (`self.ProjectileMovement`))
  (if (`self.ReduceSpeed`)
    (set `MovementComponent.Velocity` (`KismetMathLibrary.VInterpTo` (`MovementComponent.Velocity` _projectilemovement) (0.0 0.0 0.0) DeltaSeconds (`self.ReduceSpeedRate`)) _projectilemovement)))