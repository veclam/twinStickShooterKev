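; Demo actor for the Stylized Slashes pack that spawns ground slash VFX actors at a fire point for preview.
; T and R cycle through the VFX class list, clearing spawned effects, and F fires the current one.
; An automatic mode disables those keys and instead loops spawning on a timer, with delayed cleanup of spawned actors.
; An optional HUD widget displays the selected effect's name.
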(event `self.ReceiveBeginPlay`
  (`|ExecutionSequence`
    (:`then_0`
      (if (`self.CreateHUD`)
        (bind _returnvalue (`|CreateWidget` "/Game/StylizedSlashesVol1/Blueprints/SS_GroundSlashesHUD.SS_GroundSlashesHUD_C"))
        (bind _output_get (set `self.HUD` _returnvalue))
        (`UserWidget.AddToViewport` _output_get 0)))
    (:`then_1`
      (`self.EnableInput` (`GameplayStatics.GetPlayerController` 0))
      (bind _output_get_2 (set `self.CurrentVFX` (`|GetArrayItem` (`self.VFXs`))))
      (`self.RefreshVfxName` _output_get_2)
      (if (`self.ShootAutomatically`)
        (`self.SpawnGroundSlash` :!label _label)
        (`KismetSystemLibrary.Delay` 2.0)
        (goto _label)))))

(event `Key|T`
  (params (Key :type "Key Structure"))
  (:`Pressed`
    (if (not (`self.ShootAutomatically`))
      (`self.NextVFX`))))

(event `Key|R`
  (params (Key :type "Key Structure"))
  (:`Pressed`
    (if (not (`self.ShootAutomatically`))
      (`self.PreviousVFX`))))

(event `Key|F`
  (params (Key :type "Key Structure"))
  (:`Pressed`
    (if (not (`self.ShootAutomatically`))
      (`self.SpawnGroundSlash`))))

(event `SpawnGroundSlash`
  (bind _returnvalue (`|SpawnActorFromClass` (`self.CurrentVFX`) (`self.GetTransform` (`self.FirePoint`)) "Undefined" "SelectDefaultAtRuntime" null null))
  (`KismetArrayLibrary.Array_Add` (`self.SpawnedVFX`) _returnvalue)
  (if (`self.ShootAutomatically`)
    (`KismetSystemLibrary.Delay` 4.0)
    (for _array_element (`self.SpawnedVFX`)
      (`self.K2_DestroyActor` _array_element))
    (`KismetArrayLibrary.Array_Clear` (`self.SpawnedVFX`))))

(event `NextVFX`
  (if (== (`self.index`) (- (`KismetArrayLibrary.Array_Length` (`self.VFXs`)) 1))
    (set `self.index` 0)
    (else
      (set `self.index` (+ (`self.index`) 1))))
  (bind _output_get (set `self.CurrentVFX` (`|GetArrayItem` (`self.VFXs`) (`self.index`))))
  (for _array_element (`self.SpawnedVFX`)
    (`self.K2_DestroyActor` _array_element))
  (`KismetArrayLibrary.Array_Clear` (`self.SpawnedVFX`))
  (`self.RefreshVfxName` _output_get))

(event `PreviousVFX`
  (if (== (`self.index`) 0)
    (set `self.index` (- (`KismetArrayLibrary.Array_Length` (`self.VFXs`)) 1))
    (else
      (set `self.index` (- (`self.index`) 1))))
  (bind _output_get (set `self.CurrentVFX` (`|GetArrayItem` (`self.VFXs`) (`self.index`))))
  (for _array_element (`self.SpawnedVFX`)
    (`self.K2_DestroyActor` _array_element))
  (`KismetArrayLibrary.Array_Clear` (`self.SpawnedVFX`))
  (`self.RefreshVfxName` _output_get))

(event `RefreshVfxName`
  (params (GroundSlash :type "/Game/StylizedSlashesVol1/Blueprints/BP_GroundSlashParent Class Reference"))
  (if (`self.CreateHUD`)
    (`/Game/StylizedSlashesVol1/Blueprints/SS_GroundSlashesHUD.SetVfxName` (`self.HUD`) (`KismetSystemLibrary.GetClassDisplayName` GroundSlash))))

(fn `UserConstructionScript`)